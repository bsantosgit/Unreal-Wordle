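; BP_UWTile is a letter tile actor that animates feedback for incorrect and submitted letters.
; An incorrect-letter error plays a timeline that offsets the mesh side to side along local Y, at a configurable play rate.
; Submitting a letter flips the mesh 180 degrees via a timeline, with a timer swapping in the supplied material halfway through.
; The construction script disables shadow casting on the front and back widgets.
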(event `self.ReceiveBeginPlay`
  (`parent.ReceiveBeginPlay`)
  (`TimelineComponent.SetPlayRate` (`self.Timeline_IncorrectLetterError`) (`self.TimelinePlayRate`)))

(event `self.IncorrectLetterError`
  (bind (_direction _alpha) (`Timeline|Timeline_IncorrectLetterError` :!via `PlayFromStart`)
    (:`Update`
      (`SceneComponent.K2_SetRelativeLocation` (`self.TileMesh`) (`KismetMathLibrary.VLerp` (0.0 -10.0 0.0) (0.0 10.0 0.0) _alpha) false false))))

(event `self.SubmitLetter`
  (params (Material :type "MaterialInterface Object Reference"))
  (`KismetSystemLibrary.K2_SetTimerDelegate` (delegate `ChangeColors`) (/ (`TimelineComponent.GetTimelineLength` (`self.Timeline_Flip`)) 2.0))
  (bind (_direction _alpha) (`Timeline|Timeline_Flip` :!via `PlayFromStart`)
    (:`Update`
      (`SceneComponent.K2_SetRelativeRotation` (`self.TileMesh`) (`KismetMathLibrary.RLerp` (struct) (struct :`Pitch` 180.0) _alpha) false false))))

(event `ChangeColors`
  (`PrimitiveComponent.SetMaterial` (`self.TileMesh`) 0 (stale `self.SubmitLetter` Material)))

(fn `UserConstructionScript`
  (`PrimitiveComponent.SetCastShadow` (`self.WidgetFront`) false)
  (`PrimitiveComponent.SetCastShadow` (`self.WidgetBack`) false))